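; Cannonball (gülle) projectile that hits blocks and damages player characters, then destroys itself after a short timed lifetime.
; Hits on blocks call their Blocks function and increment a counter that caps further block hits at three.
; Sphere overlaps call Hasar once on character1 or character1_2, chosen by variable 01.
; Damage stops once the BeginPlay timer sets a flag, or while the hit counter equals two.
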(event `self.ReceiveBeginPlay`
  (`KismetSystemLibrary.Delay` 1.5)
  (set `self.NewVar_0` true)
  (`KismetSystemLibrary.Delay` 2.0)
  (`self.K2_DestroyActor`))

(event `self.ReceiveHit`
  (params (MyComp :type "PrimitiveComponent Object Reference") (Other :type "Actor Object Reference") (OtherComp :type "PrimitiveComponent Object Reference") (bSelfMoved :type Boolean) (HitLocation :type "Vector Structure") (HitNormal :type "Vector Structure") (NormalImpulse :type "Vector Structure") (Hit :type "HitResult Structure (by ref)"))
  (if (!= (`self.NewVar`) 3)
    (bind _asblocks (cast `/Game/Blueprints/blocks` Other))
    (`/Game/Blueprints/blocks.blocks` _asblocks)
    (set `self.NewVar` (+ (`self.NewVar`) 1))))

(event `self.Sphere.OnComponentBeginOverlap`
  (params (OverlappedComponent :type "PrimitiveComponent Object Reference") (OtherActor :type "Actor Object Reference") (OtherComp :type "PrimitiveComponent Object Reference") (OtherBodyIndex :type Integer) (bFromSweep :type Boolean) (SweepResult :type "HitResult Structure (by ref)"))
  (if (`self.NewVar_0`)
    _
    (elif (!= (`self.NewVar`) 2)
      (if (!= (`self.0,1`) 0)
        (bind _ascharacter_1 (cast `/Game/Blueprints/characters/character1` OtherActor))
        (`/Engine/EditorBlueprintResources/StandardMacros.DoOnce` false
          (:`Completed`
            (`/Game/Blueprints/characters/character1.hasar` _ascharacter_1 false 30)
            (`KismetSystemLibrary.PrintString` "sa2")))
        (else
          (bind _ascharacter_1_2 (cast `/Game/Blueprints/characters/character1_2` OtherActor))
          (`/Engine/EditorBlueprintResources/StandardMacros.DoOnce` false
            (:`Completed`
              (`/Game/Blueprints/characters/character1_2.hasar` _ascharacter_1_2 false 30)
              (`KismetSystemLibrary.PrintString` "sa3"))))))))

(fn `UserConstructionScript`)