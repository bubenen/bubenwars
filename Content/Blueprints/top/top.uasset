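; Cannon actor ("top") that characters man by entering its box, firing cannonballs ("gülle") with camera shake and sound.
; Box overlaps give character1 or character1_2 a reference to the cannon, call their Fülle and switch rotation on, reversing this on exit.
; While active, Tick flips the RotatingMovement direction whenever a pitch check chosen by NewVar passes.
; The attack event spawns the projectile at the Arrow's transform.
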(event `self.ReceiveTick`
  (params (DeltaSeconds :type "Float (single-precision)"))
  (bind _rotatingmovement (`self.RotatingMovement`))
  (bind _newvar (`self.NewVar`))
  (bind (_returnvalue_roll _returnvalue_pitch) (`KismetMathLibrary.BreakRotator` (`SceneComponent.K2_GetComponentRotation` (`self.Scene`))))
  (bind _returnvalue (> _returnvalue_pitch -10.0))
  (bind _returnvalue_2 (< _returnvalue_pitch 10.0))
  (if (`self.rotation`)
    (`ActorComponent.SetActive` _rotatingmovement true false)
    (if (`self.sa22`)
      (if (select `int` _newvar :`0` _returnvalue :`1` _returnvalue_2)
        (set `self.sa22` false)
        (set `RotatingMovementComponent.RotationRate` (struct :`Pitch` -100.0) (`self.RotatingMovement`)))
      (elif (select `int` _newvar :`0` _returnvalue :`1` _returnvalue_2)
        (set `self.sa22` true)
        (set `RotatingMovementComponent.RotationRate` (struct :`Pitch` 100.0) (`self.RotatingMovement`))))
    (else
      (`ActorComponent.SetActive` _rotatingmovement false false))))

(event `attack`
  (params (`0-1` :type Integer))
  (bind _arrow (`self.Arrow`))
  ;[1 1 1] gülleatack
  (`|SpawnActorFromClass` "/Game/Blueprints/top/_gülle._gülle_C" (`KismetMathLibrary.MakeTransform` (`SceneComponent.K2_GetComponentLocation` _arrow) (`SceneComponent.K2_GetComponentRotation` _arrow)) "Undefined" "OverrideRootScale" null `0-1` null)
  (`GameplayStatics.PlayWorldCameraShake` "/Game/sesler/shakes.shakes_C" (0.0 0.0 0.0) 2222.0 2222.0)
  (`GameplayStatics.PlaySound2D` "/Game/sesler/topatıs.topatıs" 1.0 1.0 0.0 null null))

(event `self.Box.OnComponentBeginOverlap`
  (params (OverlappedComponent :type "PrimitiveComponent Object Reference") (OtherActor :type "Actor Object Reference") (OtherComp :type "PrimitiveComponent Object Reference") (OtherBodyIndex :type Integer) (bFromSweep :type Boolean) (SweepResult :type "HitResult Structure (by ref)"))
  (bind _ascharacter_1 (cast `/Game/Blueprints/characters/character1` OtherActor)
    (:`then`
      (set `/Game/Blueprints/characters/character1.top` true _ascharacter_1)
      (set `/Game/Blueprints/characters/character1.tops` self _ascharacter_1)
      (set `self.rotation` true)
      (`/Game/Blueprints/characters/character1.fülle` _ascharacter_1 0))
    (:`CastFailed`
      (bind _ascharacter_1_2 (cast `/Game/Blueprints/characters/character1_2` OtherActor))
      (set `/Game/Blueprints/characters/character1_2.top` true _ascharacter_1_2)
      (set `/Game/Blueprints/characters/character1_2.tops` self _ascharacter_1_2)
      (set `self.rotation` true)
      (`/Game/Blueprints/characters/character1_2.fülle` _ascharacter_1_2 0))))

(event `self.Box.OnComponentEndOverlap`
  (params (OverlappedComponent :type "PrimitiveComponent Object Reference") (OtherActor :type "Actor Object Reference") (OtherComp :type "PrimitiveComponent Object Reference") (OtherBodyIndex :type Integer))
  (bind _ascharacter_1 (cast `/Game/Blueprints/characters/character1` OtherActor)
    (:`then`
      (set `/Game/Blueprints/characters/character1.top` false _ascharacter_1)
      (set `/Game/Blueprints/characters/character1.tops` null _ascharacter_1)
      (set `self.rotation` false)
      (`/Game/Blueprints/characters/character1.fülle` _ascharacter_1 1))
    (:`CastFailed`
      (bind _ascharacter_1_2 (cast `/Game/Blueprints/characters/character1_2` OtherActor))
      (set `/Game/Blueprints/characters/character1_2.top` false _ascharacter_1_2)
      (set `/Game/Blueprints/characters/character1_2.tops` null _ascharacter_1_2)
      (set `self.rotation` false)
      (`/Game/Blueprints/characters/character1_2.fülle` _ascharacter_1_2 1))))

(fn `UserConstructionScript`)