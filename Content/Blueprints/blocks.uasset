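; Block actor with a Kaleblock sprite that registers itself with the Character1 actor when its blocks event runs.
; That event disables the sprite's collision, waits briefly, teleports the block along negative Y, then adds it uniquely to the first found character's AsBlocks array.
; On BeginPlay, the Önarka (front/back) flag decides which of two black sprites is destroyed, leaving the other in place.
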(event `blocks`
  (`PrimitiveComponent.SetCollisionEnabled` (`self.kaleblock_Sprite`) "NoCollision")
  (`KismetSystemLibrary.Delay` 0.05)
  (`self.K2_SetActorLocation` (- (`self.K2_GetActorLocation`) (0.0 20.0 0.0)) false true)
  (bind _outactors (`GameplayStatics.GetAllActorsOfClass` "/Game/Blueprints/characters/character1.character1_C"))
  (`KismetArrayLibrary.Array_AddUnique` (`/Game/Blueprints/characters/character1.As Blocks` (`|GetArrayItem` _outactors)) self))

(event `self.ReceiveBeginPlay`
  (if (`self.önarka`)
    (`ActorComponent.K2_DestroyComponent` (`self.black_Sprite1`))
    (else
      (`ActorComponent.K2_DestroyComponent` (`self.black_Sprite`)))))

(fn `UserConstructionScript`)