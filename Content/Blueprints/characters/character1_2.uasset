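; Paper2D player character for a side-view versus fighter, battling a "player1" opponent who scores when this character dies and respawns.
; Custom events drive movement, limited jumps with a spin, block placing underfoot, and either a timeline-animated sword lunge or an ammo-limited cannon shot.
; Hits apply knockback, camera shake and widget feedback, with an overlap box gating sword damage.
; Overlapped pickups grant health, cannonballs or temporary double jump, or call the opponent's ResetBlock.
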(event `self.ReceiveTick`
  (params (DeltaSeconds :type "Float (single-precision)"))
  ;[0 1 0.1312] event tick
  (`self.NewFunction`)
  (if (`self.damage`)
    (`PaperFlipbookComponent.SetFlipbook` (`self.idle`) "/Game/sprite/damage/damege.damege")))

(event `hasar`
  (params (NewParam :type Boolean) (NewParam2 :type Integer))
  (bind _newvar (`self.NewVar`))
  (bind (_returnvalue_location _returnvalue_rotation) (`KismetMathLibrary.BreakTransform` (`SceneComponent.K2_GetComponentToWorld` (`self.CapsuleComponent`))))
  ;[1 1 1] hasar yeme ve ölme
  (if NewParam
    (`self.LaunchCharacter` (-155.0 0.0 155.0))
    (else
      (`self.LaunchCharacter` (155.0 0.0 155.0))))
  (`GameplayStatics.PlayWorldCameraShake` "/Game/sesler/shakes.shakes_C" (0.0 0.0 0.0) 22222.0 22222.0)
  (`GameplayStatics.PlaySound2D` "/Game/sesler/hasa1_Cue.hasa1_Cue" 1.0 1.0 0.0 null null)
  (set `self.heal` (- (`self.heal`) NewParam2))
  (bind _asc_1can_2 (cast `/Game/Blueprints/widget/c1can_2` (`WidgetComponent.GetWidget` (`self.Widget`))))
  (`UserWidget.PlayAnimation` _asc_1can_2 (`/Game/Blueprints/widget/c1can_2.sasasa` _asc_1can_2) 0.0 1 "Forward" 1.0 false)
  (`|ExecutionSequence`
    (:`then_0`
      (if (<= (`self.heal`) 0)
        (set `/Game/Blueprints/characters/character1.score` (+ (`/Game/Blueprints/characters/character1.score` _newvar) 1) _newvar)
        (`GameplayStatics.PlaySound2D` "/Game/sesler/coin.coin" 1.0 1.0 0.0 null null)
        (`|SpawnActorFromClass` "/Game/Blueprints/dead.dead_C" (`KismetMathLibrary.MakeTransform` _returnvalue_location _returnvalue_rotation (1.2 1.2 1.2)) "AlwaysSpawn" "OverrideRootScale" null null)
        (`self.K2_SetActorLocation` (0.0 -20.0 400.0))
        (set `CharacterMovementComponent.GravityScale` 0.1 (`self.CharacterMovement`))
        (`NavMovementComponent.StopActiveMovement` (`self.CharacterMovement`))
        (`KismetSystemLibrary.Delay` 2.0)
        (`self.K2_SetActorLocation` (180.753586 0.0 187.732835) false true)
        (set `self.heal` 100)
        (set `CharacterMovementComponent.GravityScale` 2.0 (`self.CharacterMovement`))))
    (:`then_1`
      (set `self.damage` true)
      (`KismetSystemLibrary.Delay` 0.2)
      (set `self.damage` false))))

(event `attack`
  ;[1 1 1] Kılıc ve hülle attack
  (if (`self.top`)
    (if (not (== (`self.gülle`) 0))
      (`/Engine/EditorBlueprintResources/StandardMacros.DoOnce` false :!label _label
        (:`Completed`
          (`/Game/Blueprints/top/top.attack` (`self.tops`) 1)
          (set `self.gülle` (- (`self.gülle`) 1))
          (`KismetSystemLibrary.Delay` 0.5)
          (goto _label :!via `Reset`))))
    (else
      (`/Engine/EditorBlueprintResources/StandardMacros.DoOnce` false :!label _label_2
        (:`Completed`
          (`self.LaunchCharacter` (select `bool` (`self.sağsol?`) :`false` (155.0 0.0 0.0) :`true` (-155.0 0.0 0.0) :!type "Vector Structure"))
          (`GameplayStatics.PlaySound2D` "/Game/sesler/attack.attack" 1.0 1.0 0.0 null null)
          (if (`self.attack?`)
            (`/Game/Blueprints/characters/character1.hasar` (`self.NewVar`) (`self.sağsol?`) 10)
            (bind (_direction _newtrack_0) (`Timeline|Timeline_0` :!via `PlayFromStart` :!label _label_3)
              (:`Update`
                (`SceneComponent.K2_SetRelativeLocationAndRotation` (`self.PaperSprite`) (`KismetMathLibrary.VLerp` (0.559787 1.879963 -2.510507) (5.527334 1.326543 -7.975956) _newtrack_0) (select `bool` (`self.sağsol?`) :`false` (`KismetMathLibrary.RLerp` (struct) (struct :`Pitch` -90.0) _newtrack_0) :`true` (`KismetMathLibrary.RLerp` (struct :`Yaw` 180.0) (struct :`Pitch` -90.0 :`Yaw` 180.0) _newtrack_0)) false false))
              (:`Finished`
                (goto _label_2 :!via `Reset`)))
            (else
              (goto _label_3 :!via `PlayFromStart`))))))))

(event `sağsol`
  (params (NewParam :type "Float (double-precision)"))
  ;[1 1 1] sağ ve sol
  (`self.AddMovementInput` (1.0 0.0 0.0) NewParam)
  (`/Engine/EditorBlueprintResources/StandardMacros.CompareFloat` NewParam
    (:`>`
      (`SceneComponent.K2_SetWorldRotation` (`self.idle`) (`KismetMathLibrary.MakeRotator` 0.0) false false)
      (`SceneComponent.K2_SetWorldRotation` (`self.PaperSprite`) (`KismetMathLibrary.MakeRotator` 0.0) false false)
      (`SceneComponent.K2_SetWorldRotation` (`self.Scene`) (`KismetMathLibrary.MakeRotator` 0.0) false false)
      (set `self.sağsol?` false))
    (:`<`
      (`SceneComponent.K2_SetWorldRotation` (`self.idle`) (`KismetMathLibrary.MakeRotator` 0.0 0.0 180.0) false false)
      (`SceneComponent.K2_SetWorldRotation` (`self.PaperSprite`) (`KismetMathLibrary.MakeRotator` 0.0 0.0 180.0) false false)
      (`SceneComponent.K2_SetWorldRotation` (`self.Scene`) (`KismetMathLibrary.MakeRotator` 0.0 0.0 180.0) false false)
      (set `self.sağsol?` true))))

(event `fülle`
  (params (`0-1` :type Integer))
  ;[1 1 1] gülle info widget
  (bind _asc_1can_2 (cast `/Game/Blueprints/widget/c1can_2` (`WidgetComponent.GetWidget` (`self.Widget`))))
  (switch `int` `0-1`
    (:`0`
      (bind `_gülle` (`/Game/Blueprints/widget/c1can_2.gülle` _asc_1can_2))
      (`UserWidget.PlayAnimationReverse` _asc_1can_2 `_gülle` 1.0 false))
    (:`1`
      (`UserWidget.PlayAnimationForward` _asc_1can_2 `_gülle` 1.0 false))))

(event `jumps`
  (bind `_sağsol_` (`self.sağsol?`))
  ;[1 1 1] jumps
  (bind _counter (`/Engine/EditorBlueprintResources/StandardMacros.Do N` (`self.jumplimit`) :!label _label_4)
    (:`Exit`
      (`self.LaunchCharacter` (`KismetMathLibrary.MakeVector` 0.0 0.0 (`CharacterMovementComponent.JumpZVelocity` (`self.CharacterMovement`))) false true)
      (if (`NavMovementComponent.IsFalling` (`self.CharacterMovement`))
        (if (== _counter 2)
          (`GameplayStatics.PlaySound2D` "/Game/sesler/jump.jump" 0.8 2.0 0.0 null null)
          (bind (_direction _newtrack_0) (`Timeline|Timeline_1` :!via `PlayFromStart`)
            (:`Update`
              (`SceneComponent.K2_SetRelativeRotation` (`self.idle`) (`KismetMathLibrary.RLerp` (select `bool` `_sağsol_` :`true` (struct :`Yaw` 180.0) :!type "Rotator Structure") (`KismetMathLibrary.SelectRotator` (struct :`Pitch` 360.0 :`Yaw` 180.0) (struct :`Pitch` 360.0) `_sağsol_`) _newtrack_0) false false))))
        (else
          (`GameplayStatics.PlaySound2D` "/Game/sesler/jump.jump" 0.8 2.0 0.0 null null))))))

(event `playanim`
  ;[1 1 1] kılıck walk anim
  (`/Engine/EditorBlueprintResources/StandardMacros.DoOnce` false :!label _label_5
    (:`Completed`
      (bind (_direction _newtrack_0) (`Timeline|Timeline` :!via `PlayFromStart`)
        (:`Update`
          (`SceneComponent.K2_SetRelativeLocation` (`self.PaperSprite`) (`KismetMathLibrary.VLerp` (0.816548 1.879963 -2.510507) (0.559787 1.879963 -4.462946) _newtrack_0) false false))
        (:`Finished`
          (goto _label_5 :!via `Reset`))))))

(event `self.OnLanded`
  (params (Hit :type "HitResult Structure (by ref)"))
  ;[1 1 1] jumps
  (goto _label_4 :!via `Reset`))

(event `down`
  (bind _location (.location (`self.GetTransform`)))
  (bind _returnvalue (`KismetMathLibrary.MakeVector_NetQuantize` (.x _location) (.y _location) (- (.z _location) 20.0)))
  ;[1 1 1] blocks
  (bind (_outhit _returnvalue_2) (`KismetSystemLibrary.CapsuleTraceSingle` _location _returnvalue 6.0 6.0 "TraceTypeQuery1"))
  (if (not _returnvalue_2)
    (`|SpawnActorFromClass` "/Game/Blueprints/block_2.block_2_C" (`KismetMathLibrary.MakeTransform` _returnvalue (.rotation (`self.GetTransform`)) (.scale (`self.GetTransform`))) "Undefined" "OverrideRootScale" null null)
    (`GameplayStatics.PlaySound2D` "/Game/sesler/block.block" 1.4 1.0 0.0 null null)))

(event `self.Box1.OnComponentBeginOverlap`
  (params (OverlappedComponent :type "PrimitiveComponent Object Reference") (OtherActor :type "Actor Object Reference") (OtherComp :type "PrimitiveComponent Object Reference") (OtherBodyIndex :type Integer) (bFromSweep :type Boolean) (SweepResult :type "HitResult Structure (by ref)"))
  ;[1 1 1] kutudestroy particle
  (bind _asreset (cast `/Game/Blueprints/loot/reset` OtherActor))
  (switch `int` (`/Game/Blueprints/loot/reset.NewVar` _asreset)
    (:`0`
      (`self.NewFunction_0`)
      (bind _location (.location (`SceneComponent.K2_GetComponentToWorld` (`/Game/Blueprints/loot/reset.resetb_Sprite` _asreset))))
      (bind _rotation (.rotation (`SceneComponent.K2_GetComponentToWorld` (`/Game/Blueprints/loot/reset.resetb_Sprite` _asreset))))
      (`|SpawnActorFromClass` "/Game/Blueprints/loot/particlew.particlew_C" (`KismetMathLibrary.MakeTransform` _location _rotation (1.4 1.4 1.4)) "AdjustIfPossibleButAlwaysSpawn" "OverrideRootScale" null 0 null)
      (`self.K2_DestroyActor` OtherActor :!label _label_6)
      (`GameplayStatics.PlaySound2D` "/Game/sesler/kutu.kutu" 1.0 1.0 0.2 null null))
    (:`1`
      (`/Game/Blueprints/characters/character1.reset block` (`self.NewVar`))
      (`|SpawnActorFromClass` "/Game/Blueprints/loot/particlergre.particlergre_C" (`KismetMathLibrary.MakeTransform` _location _rotation (1.4 1.4 1.4)) "AdjustIfPossibleButAlwaysSpawn" "OverrideRootScale" null 0 null)
      (goto _label_6))
    (:`2`
      (set `self.gülle` (+ (`self.gülle`) 2))
      (`|SpawnActorFromClass` "/Game/Blueprints/loot/particleb.particleb_C" (`KismetMathLibrary.MakeTransform` _location _rotation (1.4 1.4 1.4)) "AdjustIfPossibleButAlwaysSpawn" "OverrideRootScale" null 0 null)
      (goto _label_6))
    (:`3`
      (`|SpawnActorFromClass` "/Game/Blueprints/loot/particlenergy.particlenergy_C" (`KismetMathLibrary.MakeTransform` _location _rotation (1.4 1.4 1.4)) "AdjustIfPossibleButAlwaysSpawn" "OverrideRootScale" null 0 null)
      (`|ExecutionSequence`
        (:`then_0`
          (set `self.jumplimit` 2)
          (`KismetSystemLibrary.Delay` 8.0)
          (set `self.jumplimit` 1))
        (:`then_1`
          (goto _label_6))))))

(event `self.Box.OnComponentBeginOverlap`
  (params (OverlappedComponent :type "PrimitiveComponent Object Reference") (OtherActor :type "Actor Object Reference") (OtherComp :type "PrimitiveComponent Object Reference") (OtherBodyIndex :type Integer) (bFromSweep :type Boolean) (SweepResult :type "HitResult Structure (by ref)"))
  (bind _componenttags (`ActorComponent.ComponentTags` OtherComp))
  ;[1 1 1] attack control
  (if (`KismetArrayLibrary.Array_IsValidIndex` _componenttags)
    (if (== (`|GetArrayItem` _componenttags) "player1")
      (set `self.attack?` true))))

(event `self.Box.OnComponentEndOverlap`
  (params (OverlappedComponent :type "PrimitiveComponent Object Reference") (OtherActor :type "Actor Object Reference") (OtherComp :type "PrimitiveComponent Object Reference") (OtherBodyIndex :type Integer))
  (bind _componenttags (`ActorComponent.ComponentTags` OtherComp))
  ;[1 1 1] attack control
  (if (`KismetArrayLibrary.Array_IsValidIndex` _componenttags)
    (if (== (`|GetArrayItem` _componenttags) "player1")
      (set `self.attack?` false))))

(fn `NewFunction`
  (if (!= (`KismetMathLibrary.VSize` (`self.GetVelocity`)) 0.0)
    (`PaperFlipbookComponent.SetFlipbook` (`self.idle`) "/Game/sprite/character1/run.run")
    (`self.playanim`)
    (else
      (`PaperFlipbookComponent.SetFlipbook` (`self.idle`) "/Game/sprite/idle/run.run"))))

(fn `NewFunction_0`
  (bind _returnvalue (`WidgetComponent.GetWidget` (`self.Widget`)))
  (set `self.heal` (+ (`self.heal`) 20))
  (bind _asc_1can (cast `/Game/Blueprints/widget/c1can` _returnvalue))
  (`UserWidget.PlayAnimation` _returnvalue (`/Game/Blueprints/widget/c1can.sasasa` _asc_1can) 0.0 1 "Forward" 1.0 false))

(fn `UserConstructionScript`)