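; Short-lived jump particle sprite (çimen, "grass") that rises and fades out, then destroys its actor.
; On BeginPlay a surface switch tints it white for Cimen or near-black for Block, destroys it otherwise, and picks a random sprite.
; A timeline lifts the sprite slightly, feeding its captured relative location into SetWorldLocation, and lerps its current color toward transparent.
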(event `self.ReceiveBeginPlay`
  (bind _relative_location (`self.Relative Location`))
  (bind _partjump1_sprite (`self.partjump1_Sprite`))
  (bind _partjump1_sprite_2 (`self.partjump1_Sprite`))
  (switch `name` (`self.2`)
    (:`Default`
      (`self.K2_DestroyActor`))
    (:`cimen`
      (`PaperSpriteComponent.SetSpriteColor` _partjump1_sprite_2 (struct :`R` 1.0 :`G` 1.0 :`B` 1.0 :`A` 1.0))
      (set `self.NewVar_0` 0)
      (`PaperSpriteComponent.SetSprite` (`self.partjump1_Sprite`) (`KismetArrayLibrary.Array_Random` (`self.NewVar`)) :!label _label)
      (set `self.Relative Location` (`SceneComponent.RelativeLocation` (`self.partjump1_Sprite`)))
      (bind (_direction _newtrack_0) (`Timeline|Timeline`)
        (:`Update`
          (`SceneComponent.K2_SetWorldLocation` (`self.partjump1_Sprite`) (`KismetMathLibrary.VLerp` _relative_location (+ _relative_location (0.0 0.0 10.0)) _newtrack_0) false false)
          (`PaperSpriteComponent.SetSpriteColor` _partjump1_sprite (`KismetMathLibrary.LinearColorLerp` (`PaperSpriteComponent.SpriteColor` _partjump1_sprite) (select `int` (`self.NewVar_0`) :`0` (struct :`R` 1.0 :`G` 1.0 :`B` 1.0) :`1` (struct) :!type "LinearColor Structure") _newtrack_0)))
        (:`Finished`
          (`self.K2_DestroyActor`))))
    (:`block`
      (`PaperSpriteComponent.SetSpriteColor` _partjump1_sprite_2 (struct :`R` 0.078125 :`G` 0.078125 :`B` 0.078125 :`A` 1.0))
      (set `self.NewVar_0` 1)
      (goto _label))))

(fn `UserConstructionScript`)